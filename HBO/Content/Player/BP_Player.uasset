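; First-person player character handling movement, interaction, shooting through a child-actor gun, FMOD audio, and health and hunger shown on the HUD.
; A posture state (stand, crouch, crawl, sprint) scales move, look and footstep rates, with box-trace-checked timeline lerps resizing capsule and eye height.
; Sprinting jumps become dives into crawl.
; Hunger drains on a delay loop, then applies damage at zero; damage shakes the camera, and death reloads the level.
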(event Custom|EventHungerRestore
  (params (HungerDelta :type Float%20%28double-precision%29))
  ;[0 0 0] Player Stat Modifications
  ;;[0.4072 0.227 0.09531] Hunger Restore Event
  (bind _returnvalue (PlayerData|ReduceHunger HungerDelta))
  (Default|SetHunger (Variables|Components|GetWBP_HUD) _returnvalue 1e+02))

(event Custom|EventHealthRestore
  (params (Health%20Delta :type Float%20%28double-precision%29))
  ;[0 0 0] Player Stat Modifications
  ;;[0.4072 0.09306 0.162] Health Restore Event
  (PlayerData|RestoreHealth Health%20Delta)
  (PlayerData|UpdateHealthbar))

(event Custom|PostureAnimEvent
  (params (StartPosture :type E_PlayerMoveState%20Enum :default "NewEnumerator0") (EndPosture :type E_PlayerMoveState%20Enum :default "NewEnumerator0") (LengthSelect :type E_AnimLengthSelector%20Enum :default "NewEnumerator0"))
  ;[0.7496 1 0.8122 1 26] Animation Events
  ;;[0.18 0.3 0.3] Player Posture Change Event
  (bind _blocked (PlayerPosture|GetCanStandup StartPosture EndPosture))
  (if (not _blocked)
    (switch Utilities|FlowControl|Switch|SwitchonE_AnimLengthSelector LengthSelect
      (:NewEnumerator4
        (Utilities|FlowControl|Sequence
          (:then_0
            (PlayerPosture|SetPlayerHeight (Variables|Default|GetC_Player) (Variables|Collision|GetCapsuleComponent) StartPosture EndPosture (Utilities|MLerpAlphaSelect 1.0 (stale _length__0_3) (stale _length__0_5) LengthSelect) :!label _label))
          (:then_1
            (PlayerPosture|SetPostureandNotify EndPosture :!label _label_2))))
      (:NewEnumerator0
        (bind (_direction _length__0_3 _length__0_5) (Timeline|ZeroToOneCurves PlayFromStart)
          (:Update
            (goto _label))
          (:0.3%20Finished
            (goto _label_2))))
      (:NewEnumerator1
        (Timeline|ZeroToOneCurves PlayFromStart))
      (:NewEnumerator2
        (Timeline|ZeroToOneCurves PlayFromStart))
      (:NewEnumerator3
        (Timeline|ZeroToOneCurves PlayFromStart)))))

(event Custom|CameraShake
  (bind _returnvalue (Pawn|GetControlRotation :!class /Script/Engine.Pawn))
  (bind _c_player (Variables|Default|GetC_Player))
  ;[0.7496 1 0.8122 1 26] Animation Events
  ;;[0.18 0.3 0.3] Camera Shake
  (Utilities|FlowControl|DoOnce false :!label _label
    (:Completed
      (Variables|/Script/Engine.CameraComponent|SetbUsePawnControlRotation (Variables|Default|GetC_Player) false)
      (Variables|PlayerData|SetCameraShakeDelta (Math|Float|SelectFloat (Variables|PlayerData|GetCameraShakeDelta) (* (Variables|PlayerData|GetCameraShakeDelta) -1.0) (Math|Random|RandomBool)))
      (bind _zerotoone (Timeline|CameraShakeTimeline PlayFromStart)
        (:Update
          (Transformation|SetWorldRotation _c_player (Math|Rotator|MakeRotator (+ (Math|Float|Lerp 0.0 (Variables|PlayerData|GetCameraShakeDelta) _zerotoone) (.roll _returnvalue)) (.pitch _returnvalue) (.yaw _returnvalue)) false false))
        (:Finished
          (Variables|/Script/Engine.CameraComponent|SetbUsePawnControlRotation _c_player true)
          (goto _label Reset))))))

(event Custom|PostureUpdate
  (params (New%20Posture :type E_PlayerMoveState%20Enum :default "NewEnumerator0"))
  (bind _returnvalue (Utilities|MGetSpeedfromPosture New%20Posture))
  (bind _returnvalue_2 (- _returnvalue 0.1))
  (bind _returnvalue_3 (- 1.0 _returnvalue_2))
  ;[0 0 1] Player Movement Speed
  (Utilities|FlowControl|Sequence
    (:then_0
      ;;[0 0 0.6] Set FMOD Movement Speed Function
      (Default|SetFMODParameter-MovementSpeed (Variables|Default|GetAC_FMODAudioComponent) (Variables|Default|GetFMOD_PLYR_FTS_Event) (Utilities|MGetSpeedfromPosture New%20Posture)))
    (:then_1
      ;;[0 0 0.6] Update Footstep Sounds By Player State
      (Utilities|FlowControl|Delay (Utilities|Time|GetTimerRemainingTimebyHandle (Variables|WwiseAudio|GetPlayerFootstepTimer)))
      (Utilities|Time|ClearandInvalidateTimerbyHandle (Variables|WwiseAudio|GetPlayerFootstepTimer))
      (bind _returnvalue_4 (Utilities|Time|SetTimerbyFunctionName 0 "PlayFootstepSound" (Math|Float|Clamp(Float) _returnvalue_3 0.3 0.7) true (* _returnvalue_3 -1.0)))
      (Variables|WwiseAudio|SetPlayerFootstepTimer _returnvalue_4))))

(event Custom|HungerDepreciation
  ;[0 0 0] Player Stat Modifications
  ;;[1 0.5653 0.236] Hunger Depreciation Loop
  (Utilities|FlowControl|Delay (Variables|PlayerStats|GetHungerTimeDelta) :!label _label)
  (Utilities|MIsPlayerHungry
    (:Hungry
      (PlayerData|ReduceHealthbyHunger))
    (:Not%20Hungry
      (PlayerData|IncreaseHunger (Variables|PlayerStats|GetPlayerHungerDelta) (Variables|PlayerStats|GetPlayerHunger))
      (Default|SetHunger (Variables|Components|GetWBP_HUD) (Variables|PlayerStats|GetPlayerHunger) 1e+02)
      (goto _label))))

(event Custom|PlayFootsteps
  (bind _playerposture (Variables|PlayerPosture|GetPlayerPosture))
  (bind _returnvalue (Utilities|MGetSpeedfromPosture _playerposture))
  (bind _returnvalue_2 (- _returnvalue 0.1))
  (bind _returnvalue_3 (- 1.0 _returnvalue_2))
  ;[0 0 1] Player Footsteps
  (if (not (Utilities|Time|IsValidTimerHandle (Variables|WwiseAudio|GetPlayerFootstepTimer)))
    (bind _returnvalue_4 (Utilities|Time|SetTimerbyFunctionName 0 "PlayFootstepSound" (Math|Float|Clamp(Float) _returnvalue_3 0.3 0.7) true (* _returnvalue_3 -1.0)))
    (Variables|WwiseAudio|SetPlayerFootstepTimer _returnvalue_4)))

(event Custom|StopFootsteps
  ;[0 0 1] Player Footsteps
  (Utilities|Time|ClearandInvalidateTimerbyHandle (Variables|WwiseAudio|GetPlayerFootstepTimer)))

(event Input|EnhancedActionEvents|EnhancedInputActionIA_CrouchCrawl
  (params (ActionValue :type Boolean) (ElapsedSeconds :type Float%20%28double-precision%29) (TriggeredSeconds :type Float%20%28double-precision%29) (InputAction :type Input%20Action%20Object%20Reference :default "/Game/Player/Input/Actions/IA_CrouchCrawl.IA_CrouchCrawl"))
  (bind _playerposture (Variables|PlayerPosture|GetPlayerPosture))
  ;[0.18 0.3 0.3] Crouch/Crawl
  ;;[0.07 0.28 0.25] Enter Crawl
  (if (not (Audio|Components|Audio|IsPlaying (Variables|Default|GetZeroToOneCurves)))
    (Variables|PlayerPosture|SetPrevPlayerPosture _playerposture)
    (switch Utilities|FlowControl|Switch|SwitchonE_PlayerMoveState _playerposture
      (:NewEnumerator0
        (Variables|PlayerPosture|SetTargetPlayerPosture "NewEnumerator2" :!label _label))
      (:NewEnumerator1
        (goto _label))
      (:NewEnumerator2
        (Variables|PlayerPosture|SetTargetPlayerPosture "NewEnumerator0")))
    ;;[0.07 0.28 0.25] Stand Up Anim - Normal
    (CallFunction|PostureAnimEvent (Variables|PlayerPosture|GetPrevPlayerPosture) (Variables|PlayerPosture|GetTargetPlayerPosture) "NewEnumerator0")))

(event Input|EnhancedActionEvents|EnhancedInputActionIA_CrouchCrawl
  (params (ActionValue :type Boolean) (ElapsedSeconds :type Float%20%28double-precision%29) (TriggeredSeconds :type Float%20%28double-precision%29) (InputAction :type Input%20Action%20Object%20Reference :default "/Game/Player/Input/Actions/IA_CrouchCrawl.IA_CrouchCrawl"))
  (bind _playerposture (Variables|PlayerPosture|GetPlayerPosture))
  ;[0.18 0.3 0.3] Crouch/Crawl
  ;;[0.07 0.28 0.25] Crouch Toggle
  (:Canceled
    (if (not (Audio|Components|Audio|IsPlaying (Variables|Default|GetZeroToOneCurves)))
      (Variables|PlayerPosture|SetPrevPlayerPosture _playerposture)
      (switch Utilities|FlowControl|Switch|SwitchonE_PlayerMoveState _playerposture
        (:NewEnumerator0
          (Variables|PlayerPosture|SetTargetPlayerPosture "NewEnumerator1" :!label _label))
        (:NewEnumerator1
          (Variables|PlayerPosture|SetTargetPlayerPosture "NewEnumerator0"))
        (:NewEnumerator2
          (goto _label)))
      ;;[0.07 0.28 0.25] Stand Up Anim - Normal
      (CallFunction|PostureAnimEvent (Variables|PlayerPosture|GetPrevPlayerPosture) (Variables|PlayerPosture|GetTargetPlayerPosture) "NewEnumerator0"))))

(event Input|EnhancedActionEvents|EnhancedInputActionIA_Aim
  (params (ActionValue :type Boolean) (ElapsedSeconds :type Float%20%28double-precision%29) (TriggeredSeconds :type Float%20%28double-precision%29) (InputAction :type Input%20Action%20Object%20Reference :default "/Game/Player/Input/Actions/IA_Aim.IA_Aim"))
  (bind _guncomponent (Variables|Default|GetGunComponent))
  (bind _childactor (Variables|/Script/Engine.ChildActorComponent|GetChildActor _guncomponent))
  ;[1 1 1] Use Weapons
  (:Started
    (bind _asbp_gun (Utilities|Casting|CastToBP_Gun _childactor))
    (Default|SetADS _asbp_gun true))
  (:Completed
    (bind _asbp_gun_2 (Utilities|Casting|CastToBP_Gun _childactor))
    (Default|SetADS _asbp_gun_2 false)))

(event Input|EnhancedActionEvents|EnhancedInputActionIA_Camera
  (params (ActionValue :type Vector%202D%20Structure) (ElapsedSeconds :type Float%20%28double-precision%29) (TriggeredSeconds :type Float%20%28double-precision%29) (InputAction :type Input%20Action%20Object%20Reference :default "/Game/Player/Input/Actions/IA_Camera.IA_Camera"))
  (bind _playerposture (Variables|PlayerPosture|GetPlayerPosture))
  (bind (_yawout _pitchout) (Utilities|MLookSpeedfromPosture (.x ActionValue) (.y ActionValue) _playerposture))
  ;[0.1804 0.298 0.302] Camera Controls
  (Pawn|Input|AddControllerYawInput _yawout)
  (Pawn|Input|AddControllerPitchInput _pitchout))

(event Input|EnhancedActionEvents|EnhancedInputActionIA_Move
  (params (ActionValue :type Vector%202D%20Structure) (ElapsedSeconds :type Float%20%28double-precision%29) (TriggeredSeconds :type Float%20%28double-precision%29) (InputAction :type Input%20Action%20Object%20Reference :default "/Game/Player/Input/Actions/IA_Move.IA_Move"))
  (bind _self self)
  (bind _ac_fmodaudiocomponent (Variables|Default|GetAC_FMODAudioComponent))
  (bind _playerposture (Variables|PlayerPosture|GetPlayerPosture))
  (bind (_outspeedx _outspeedy) (Utilities|MMoveSpeedfromPosture _playerposture (.x ActionValue) (.y ActionValue)))
  ;[0.18 0.3 0.3] Movement
  (:Triggered
    ;;[0.07 0.28 0.25] Lateral Movement
    (Pawn|Input|AddMovementInput (Math|Vector|Normalize (Transformation|GetActorRightVector) 0.001) _outspeedx false)
    ;;[0.07 0.28 0.25] Longitudinal Movement
    (Pawn|Input|AddMovementInput (Math|Vector|Normalize (Transformation|GetActorForwardVector) 0.001) _outspeedy false))
  (:Started
    ;;[0 0 1] Play Temp Footsteps
    (bind _audio_component_reference (Default|PlayFMODEvent _ac_fmodaudiocomponent "/Game/FMOD/Events/SFX/Player/PLYR_Locomotion/PLYR_TempFootsteps.PLYR_TempFootsteps" _self))
    (bind _output_get (Variables|Default|SetFMOD_PLYR_FTS_Event _audio_component_reference))
    (Default|SetFMODParameter-MovementSpeed _ac_fmodaudiocomponent _output_get 0.6))
  (:Completed
    (Default|PlayFMODEvent _ac_fmodaudiocomponent "/Game/FMOD/Events/SFX/Player/PLYR_Locomotion/PLYR_TempFootsteps_STOP.PLYR_TempFootsteps_STOP" _self)))

(event Input|EnhancedActionEvents|EnhancedInputActionIA_Shoot
  (params (ActionValue :type Boolean) (ElapsedSeconds :type Float%20%28double-precision%29) (TriggeredSeconds :type Float%20%28double-precision%29) (InputAction :type Input%20Action%20Object%20Reference :default "/Game/Player/Input/Actions/IA_Shoot.IA_Shoot"))
  ;[1 1 1] Use Weapons
  (:Started
    (bind _asbp_gun (Utilities|Casting|CastToBP_Gun (Variables|/Script/Engine.ChildActorComponent|GetChildActor (Variables|Default|GetGunComponent))))
    (bind (_shotbullet _reload) (Default|Shoot _asbp_gun self (Variables|Default|GetC_Player)))
    (if _reload
      (Default|StartReload _asbp_gun)
      (elif (and (Variables|/Game/GameObjects/Interactables/Pickups/GunPLACEHOLDER/BP_Gun.BP_Gun_C|GetAiming _asbp_gun) _shotbullet) ; If we shot and we're aiming, apply camera recoil
        (Pawn|Input|AddControllerPitchInput (Math|Random|RandomFloatinRange (.X (Math|Vector2D|BreakVector2D (Variables|/Game/GameObjects/Interactables/Pickups/GunPLACEHOLDER/BP_Gun.BP_Gun_C|GetVerticalCamRecoilRange _asbp_gun))) (.Y (Math|Vector2D|BreakVector2D (Variables|/Game/GameObjects/Interactables/Pickups/GunPLACEHOLDER/BP_Gun.BP_Gun_C|GetVerticalCamRecoilRange _asbp_gun)))))
        (Pawn|Input|AddControllerYawInput (Math|Random|RandomFloatinRange (.X (Math|Vector2D|BreakVector2D (Variables|/Game/GameObjects/Interactables/Pickups/GunPLACEHOLDER/BP_Gun.BP_Gun_C|GetHorizontalCamRecoilRange _asbp_gun))) (.Y (Math|Vector2D|BreakVector2D (Variables|/Game/GameObjects/Interactables/Pickups/GunPLACEHOLDER/BP_Gun.BP_Gun_C|GetHorizontalCamRecoilRange _asbp_gun)))))))))

(event Input|EnhancedActionEvents|EnhancedInputActionIA_Sprint
  (params (ActionValue :type Boolean) (ElapsedSeconds :type Float%20%28double-precision%29) (TriggeredSeconds :type Float%20%28double-precision%29) (InputAction :type Input%20Action%20Object%20Reference :default "/Game/Player/Input/Actions/IA_Sprint.IA_Sprint"))
  ;[0.18 0.3 0.3] Sprinting
  (:Started
    (if (not (Audio|Components|Audio|IsPlaying (Variables|Default|GetZeroToOneCurves)))
      (bind _output_get (Variables|PlayerPosture|SetPrevPlayerPosture (Variables|PlayerPosture|GetPlayerPosture)))
      (switch Utilities|FlowControl|Switch|SwitchonE_PlayerMoveState _output_get
        (:NewEnumerator0
          (PlayerPosture|SetPostureandNotify "NewEnumerator3"))
        (:NewEnumerator1
          (Variables|PlayerPosture|SetTargetPlayerPosture "NewEnumerator3")
          ;;[0.07 0.28 0.25] Enter Sprint From Crouch
          (CallFunction|PostureAnimEvent (Variables|PlayerPosture|GetPrevPlayerPosture) (Variables|PlayerPosture|GetTargetPlayerPosture) "NewEnumerator0"))
        (:NewEnumerator2
          (Variables|PlayerPosture|SetTargetPlayerPosture "NewEnumerator3")
          ;;[0.07 0.28 0.25] Enter Sprint From Crawl
          (CallFunction|PostureAnimEvent (Variables|PlayerPosture|GetPrevPlayerPosture) (Variables|PlayerPosture|GetTargetPlayerPosture) "NewEnumerator1"))))))

(event Input|EnhancedActionEvents|EnhancedInputActionIA_Interact
  (params (ActionValue :type Boolean) (ElapsedSeconds :type Float%20%28double-precision%29) (TriggeredSeconds :type Float%20%28double-precision%29) (InputAction :type Input%20Action%20Object%20Reference :default "/Game/Player/Input/Actions/IA_Interact.IA_Interact"))
  (bind _triggerregion (Variables|Default|GetTriggerRegion))
  (bind _overlappingactors (Collision|GetOverlappingActors _triggerregion "/Game/GameObjects/Interactables/BP_InteractableObject.BP_InteractableObject_C" :!class /Script/Engine.PrimitiveComponent))
  ;[0.18 0.3 0.3] Interact
  (:Ongoing
    (Class|BPIInteract|InteractOngoing(Message) _overlappingactors))
  (:Canceled
    (Class|BPIInteract|InteractTapped(Message) _overlappingactors)))

(event Input|EnhancedActionEvents|EnhancedInputActionIA_Action
  (params (ActionValue :type Boolean) (ElapsedSeconds :type Float%20%28double-precision%29) (TriggeredSeconds :type Float%20%28double-precision%29) (InputAction :type Input%20Action%20Object%20Reference :default "/Game/Player/Input/Actions/IA_Action.IA_Action"))
  (bind _playerposture (Variables|PlayerPosture|GetPlayerPosture))
  ;[0.18 0.3 0.3] Action Button Events
  (:Started
    (switch Utilities|FlowControl|Switch|SwitchonE_PlayerMoveState _playerposture
      (:NewEnumerator0
        ;;[0.07 0.28 0.25] Hop
        (Character|Jump))
      (:NewEnumerator3
        ;;[0.07 0.28 0.25] Dive
        (PlayerActions|DiveStart)
        (Utilities|FlowControl|DoOnce true) ; enters at Reset
      )))
  (:Canceled
    (switch Utilities|FlowControl|Switch|SwitchonE_PlayerMoveState _playerposture
      (:NewEnumerator0
        (Character|StopJumping)))))

(event Input|EnhancedActionEvents|EnhancedInputActionIA_ForwardHeld
  (params (ActionValue :type Boolean) (ElapsedSeconds :type Float%20%28double-precision%29) (TriggeredSeconds :type Float%20%28double-precision%29) (InputAction :type Input%20Action%20Object%20Reference :default "/Game/Player/Input/Actions/IA_ForwardHeld.IA_ForwardHeld"))
  ;[0.18 0.3 0.3] Sprinting
  ;;[0.07 0.28 0.25] Exit Sprint
  (:Completed
    (switch Utilities|FlowControl|Switch|SwitchonE_PlayerMoveState (Variables|PlayerPosture|GetPlayerPosture)
      (:NewEnumerator3
        (PlayerPosture|SetPostureandNotify "NewEnumerator0")))))

(event Input|EnhancedActionEvents|EnhancedInputActionIA_Reload
  (params (ActionValue :type Boolean) (ElapsedSeconds :type Float%20%28double-precision%29) (TriggeredSeconds :type Float%20%28double-precision%29) (InputAction :type Input%20Action%20Object%20Reference :default "/Game/Player/Input/Actions/IA_Reload.IA_Reload"))
  ;[1 1 1] Use Weapons
  (Default|StartReload (stale Input|EnhancedActionEvents|EnhancedInputActionIA_Shoot _asbp_gun)))

(event Game|Damage|EventAnyDamage
  (params (Damage :type Float%20%28single-precision%29) (DamageType :type Damage%20Type%20Object%20Reference) (InstigatedBy :type Controller%20Object%20Reference) (DamageCauser :type Actor%20Object%20Reference))
  ;[0 0 0] Player Stat Modifications
  ;;[0.18 0.3 0.3] Damage Events
  (Utilities|FlowControl|Sequence
    (:then_0
      ;;;[1 0.2294 0.4] Update Health After Damage
      (PlayerData|ReduceHealth (Variables|PlayerStats|GetPlayerHealth) Damage)
      (PlayerData|UpdateHealthbar))
    (:then_1
      ;;;[0.07 0.28 0.25] Shake Camera
      (CallFunction|CameraShake))))

(event EventBeginPlay
  (bind _ac_fmodaudiocomponent (Variables|Default|GetAC_FMODAudioComponent))
  ;[0.1804 0.298 0.302] On Begin Play
  (Utilities|FlowControl|Sequence
    (:then_0
      ;;[0.07 0.28 0.25] Create HUD Widget Reference
      (bind _returnvalue (UserInterface|CreateWidget "/Game/UI/WBP_HUD.WBP_HUD_C"))
      (UserInterface|Viewport|AddtoViewport _returnvalue 0)
      (Variables|Components|SetWBP_HUD _returnvalue)
      (CallFunction|HungerDepreciation))
    (:then_1
      ;;[0 0 1] Play 2D Ambience
      (Default|SetFMODParameter-AreaState _ac_fmodaudiocomponent "NewEnumerator2")
      (Default|SetFMODParameter-ZoneState _ac_fmodaudiocomponent "NewEnumerator6")
      (Default|PlayFMODEvent _ac_fmodaudiocomponent "/Game/FMOD/Events/SFX/2DAmbiences/2DAMB_MainSwitch.2DAMB_MainSwitch"))))

(event EventOnLanded
  (params (Hit :type Hit%20Result%20Structure%20%28by%20ref%29))
  ;[0.18 0.3 0.3] Action Button Events
  ;;[0.07 0.28 0.25] Dive
  (Utilities|FlowControl|DoOnce true
    (:Completed
      (PlayerActions|DiveEnd))))

(fn ConstructionScript)

(fn GetCanStandup
  (params (StartState :type E_PlayerMoveState%20Enum :default "NewEnumerator0") (EndState :type E_PlayerMoveState%20Enum :default "NewEnumerator0"))
  (bind _returnvalue (Transformation|GetActorLocation))
  (bind (_eyeheight _capsulehalfheight _capsuleradius) (Utilities|MGetHeightfromPosture EndState))
  ;[0.18 0.3 0.3] Check if player can stand via box trace from previous body state towards target body state
  (switch Utilities|FlowControl|Switch|SwitchonE_PlayerMoveState StartState
    (:NewEnumerator0
      _)
    (:NewEnumerator1
      (if (Utilities|Enum|Equal(Enum) EndState "NewEnumerator2")
        _
        (else
          (bind _returnvalue_2 (Class|KismetSystemLibrary|BoxTraceSingleforObjects _returnvalue (+ _returnvalue (Math|Vector|MakeVector 0.0 0.0 (- (* _capsulehalfheight 2.0) _capsuleradius))) (Math|Vector|MakeVector _capsuleradius _capsuleradius 0.0) "0, 0, 0" (Utilities|Array|MakeArray "ObjectTypeQuery1") false (Utilities|Array|MakeArray self) "None" true :!label _label)))))
    (:NewEnumerator2
      (goto _label))
    (:NewEnumerator3
      _)
    (:NewEnumerator4
      _))
  (return _returnvalue_2))

(fn SetPlayerHeight
  (params (Camera :type Camera%20Component%20Object%20Reference%20%28by%20ref%29) (Capsule :type Capsule%20Component%20Object%20Reference) (StartState :type E_PlayerMoveState%20Enum :default "NewEnumerator0") (EndState :type E_PlayerMoveState%20Enum :default "NewEnumerator0") (Alpha :type Float%20%28double-precision%29))
  (bind (_eyeheight _capsulehalfheight) (Utilities|MGetHeightfromPosture StartState))
  (bind (_eyeheight_2 _capsulehalfheight_2) (Utilities|MGetHeightfromPosture EndState))
  ;[0.18 0.3 0.3] Body Height
  (Components|Capsule|SetCapsuleHalfHeight Capsule (Math|Float|Lerp _capsulehalfheight _capsulehalfheight_2 Alpha) true)
  ;[0.18 0.3 0.3] Body Radius
  (Components|Capsule|SetCapsuleRadius Capsule (.CapsuleRadius (Utilities|MGetHeightfromPosture (Variables|PlayerPosture|GetTargetPlayerPosture))) true)
  ;[0.18 0.3 0.3] Eyeline
  (Transformation|SetRelativeTransform Camera (Math|Transform|MakeTransform (Math|Vector|MakeVector 0.0 0.0 (Math|Float|Lerp _eyeheight _eyeheight_2 Alpha)) "0, 0, 0" "1.000000,1.000000,1.000000") false false))

(fn ReduceHealth
  (params (Player%20Health :type Float%20%28double-precision%29) (Health%20Delta :type Float%20%28double-precision%29))
  (bind _output_get (Variables|PlayerStats|SetPlayerHealth (Math|Float|Clamp(Float) (- Player%20Health Health%20Delta) 0.0 1e+02)))
  (PlayerData|IsPlayerDead _output_get))

(fn UpdateHealthbar
  (Default|SetHealth (Variables|Components|GetWBP_HUD) (Variables|PlayerStats|GetPlayerHealth) 1e+02))

(fn IncreaseHunger
  (params (A :type Float%20%28double-precision%29) (B :type Float%20%28double-precision%29))
  (Variables|PlayerStats|SetPlayerHunger (Math|Float|Clamp(Float) (- B A) 0.0 1e+02)))

(fn ReduceHealthbyHunger
  (Game|Damage|ApplyDamage (Game|Player|GetPlayerPawn 0) (Variables|PlayerStats|GetPlayerHungerDelta) 0 0))

(fn ReduceHunger
  (params (A :type Float%20%28double-precision%29))
  (Variables|PlayerStats|SetPlayerHunger (Math|Float|Clamp(Float) (+ A (Variables|PlayerStats|GetPlayerHunger)) 0.0 1e+02))
  (return (Math|Float|Clamp(Float) (+ A (Variables|PlayerStats|GetPlayerHunger)) 0.0 1e+02)))

(fn RestoreHealth
  (params (Health%20Delta :type Float%20%28double-precision%29))
  (Variables|PlayerStats|SetPlayerHealth (Math|Float|Clamp(Float) (+ Health%20Delta (Variables|PlayerStats|GetPlayerHealth)) 0.0 1e+02)))

(fn IsPlayerDead
  (params (Player%20Health :type Float%20%28double-precision%29))
  (if (<= Player%20Health 0.001)
    (bind _returnvalue (Game|GetCurrentLevelName true))
    (Game|OpenLevel(byName) (Utilities|String|StringToName _returnvalue))))

(fn SetPostureandNotify
  (params (NewPosture :type E_PlayerMoveState%20Enum :default "NewEnumerator0"))
  (bind _output_get (Variables|PlayerPosture|SetPlayerPosture NewPosture))
  (CallFunction|PostureUpdate _output_get))

(fn DiveStart
  (Input|DisableInput 0)
  (Character|LaunchCharacter (+ (* (Transformation|GetActorForwardVector) (Variables|PlayerData|GetDiveForce)) (* (Transformation|GetActorUpVector) (Variables|PlayerData|GetDiveForce))) false false)
  (CallFunction|PostureAnimEvent "NewEnumerator3" "NewEnumerator2" "NewEnumerator1"))

(fn DiveEnd
  (CallFunction|CameraShake)
  (Input|EnableInput 0))

(fn GetPosture
  (return (Variables|PlayerPosture|GetPlayerPosture)))