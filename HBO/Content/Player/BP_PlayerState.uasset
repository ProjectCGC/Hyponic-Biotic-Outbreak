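; Player state Blueprint that holds the player's health and an inventory of collected keys.
; The AnyDamage event subtracts damage from health, clamped between zero and max health and truncated to an integer.
; Inventory can be set or read as a whole, while AddToPlayerInventory adds keys uniquely and skips one specific enum value.
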(event Game|Damage|EventAnyDamage
  (params (Damage :type Float%20%28single-precision%29) (DamageType :type Damage%20Type%20Object%20Reference) (InstigatedBy :type Controller%20Object%20Reference) (DamageCauser :type Actor%20Object%20Reference))
  (Variables|Default|SetPlayerHealth (Math|Float|Truncate (Math|Float|Clamp(Float) (- (Variables|Default|GetPlayerHealth) Damage) 0.0 (Math|Conversions|ToFloat(Integer) (Variables|Default|GetMaxHealth))))))

(event EventSetPlayerInventory
  (params (NewInventory :type F%20Player%20Inventory%20Structure%20%28by%20ref%29))
  (Variables|Default|SetInventory NewInventory))

(fn ConstructionScript)

(fn AddtoPlayerInventory
  (params (NewKey :type E_KeyTypes%20Enum :default "NewEnumerator3"))
  (if (Utilities|Enum|NotEqual(Enum) NewKey "NewEnumerator3")
    (bind _returnvalue (Utilities|Array|AddUnique (Utilities|Struct|BreakF_PlayerInventory (Variables|Default|GetInventory)) NewKey))
    (return _returnvalue)))

(fn GetPlayerInventory
  (return (Variables|Default|GetInventory)))