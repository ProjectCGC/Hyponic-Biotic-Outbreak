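; Blueprint function library of math helpers for vector angles and distance, rate and time calculations.
; AngleBetweenTwoVectors normalizes both vectors and takes the arccosine of their dot product, returning degrees.
; TimeConversion solves whichever of distance, rate or time is non-positive, deriving distance from Start and End points when none is given.
; It returns all three values, or -1 for each unless exactly one is unknown.
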(fn AngleBetweenTwoVectors
  (params (V1 :type Vector) (V2 :type Vector))
  (return (Class|KismetMathLibrary|DegAcos (Math|Vector|DotProduct (Math|Vector|Normalize V1 0.001) (Math|Vector|Normalize V2 0.001)))))

(fn TimeConversion
  (params (Distance :type Float%20%28double-precision%29) (Start :type Vector) (End :type Vector) (Rate :type Float%20%28double-precision%29) (Time :type Float%20%28double-precision%29))
  (bind _returnvalue (Math|Vector|Distance(Vector) Start End))
  (bind _solvefor (LocalVariables|GetSolveFor))
  (if (> Distance 0.0)
    (LocalVariables|SetLocalDistance Distance)
    (elif (> _returnvalue 0.0)
      (LocalVariables|SetLocalDistance _returnvalue)
      (else
        (Utilities|Array|Add (LocalVariables|GetSolveFor) 1))))
  (if (> Rate 0.0)
    (LocalVariables|SetLocalRate Rate)
    (else
      (Utilities|Array|Add (LocalVariables|GetSolveFor) 2)))
  (if (> Time 0.0)
    (LocalVariables|SetLocalTime Time)
    (else
      (Utilities|Array|Add (LocalVariables|GetSolveFor) 3)))
  (if (and (== (Utilities|Array|Length _solvefor) 1) (Utilities|Array|IsValidIndex _solvefor))
    (switch int (Utilities|Array|Get(acopy) _solvefor)
      (:Default
        _)
      (:0
        _)
      (:1
        (Utilities|Array|Clear (LocalVariables|GetSolveFor))
        (return (* (LocalVariables|GetLocalTime) (LocalVariables|GetLocalRate)) (LocalVariables|GetLocalRate) (LocalVariables|GetLocalTime)))
      (:2
        (Utilities|Array|Clear (LocalVariables|GetSolveFor))
        (return (LocalVariables|GetLocalDistance) (Math|Float|SafeDivide (LocalVariables|GetLocalDistance) (LocalVariables|GetLocalTime)) (LocalVariables|GetLocalTime)))
      (:3
        (Utilities|Array|Clear (LocalVariables|GetSolveFor))
        (return (LocalVariables|GetLocalDistance) (LocalVariables|GetLocalRate) (Math|Float|SafeDivide (LocalVariables|GetLocalDistance) (LocalVariables|GetLocalRate))))))
  (Utilities|Array|Clear (LocalVariables|GetSolveFor))
  (return -1.0 -1.0 -1.0))