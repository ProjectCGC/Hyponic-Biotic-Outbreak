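; BP_InteractableObject is an interactable actor that shows a UI widget while the player is nearby.
; It hides UIWidget on BeginPlay and reveals it when the player character begins overlapping the UI_Radius component.
; When that overlap ends, it hides the widget after a short delay, without rechecking whether the player has re-entered.
; The graphs contain only this prompt visibility logic, with no interaction handling.
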(event OnComponentBeginOverlap(UI_Radius)
  (params (OverlappedComponent :type Primitive%20Component%20Object%20Reference) (OtherActor :type Actor%20Object%20Reference) (OtherComp :type Primitive%20Component%20Object%20Reference) (OtherBodyIndex :type Integer) (bFromSweep :type Boolean) (SweepResult :type Hit%20Result%20Structure%20%28by%20ref%29))
  (if (== OtherActor (Game|GetPlayerCharacter 0))
    (Rendering|SetVisibility (Variables|Default|GetUI_Widget) true true)))

(event OnComponentEndOverlap(UI_Radius)
  (params (OverlappedComponent :type Primitive%20Component%20Object%20Reference) (OtherActor :type Actor%20Object%20Reference) (OtherComp :type Primitive%20Component%20Object%20Reference) (OtherBodyIndex :type Integer))
  (if (== OtherActor (Game|GetPlayerCharacter 0))
    (Utilities|FlowControl|Delay 0.2)
    (Rendering|SetVisibility (Variables|Default|GetUI_Widget) false true)))

(event EventBeginPlay
  (Rendering|SetVisibility (Variables|Default|GetUI_Widget) false true))

(fn ConstructionScript)