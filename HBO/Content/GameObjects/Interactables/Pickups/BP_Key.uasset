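; Interactable key pickup that adds its key type to the player's inventory when tapped.
; A DoOnce-guarded InteractTapped event plays the PLYR_HealthUp FMOD event on the player pawn, passes KeyType to player state 0 via an AddToPlayerInventory message, then destroys the key.
; The key's own AddToPlayerInventory and GetPlayerInventory functions are empty stubs, and its construction script only calls the parent.
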(event EventInteractTapped
  ;[0.18 0.3 0.3] Collect Key Object
  (Utilities|FlowControl|DoOnce false
    (:Completed
      ;;[0 0 1] Audio
      (Default|PlayFMODEvent (Variables|Default|GetAC_WwiseAudioComponent) "/Game/FMOD/Events/SFX/Player/PLYR_Interaction/PLYR_HealthUp.PLYR_HealthUp" (Game|Player|GetPlayerPawn 0))
      (Class|BPIInventory|AddtoPlayerInventory(Message) (Game|GetPlayerState 0) (Variables|Default|GetKeyType))
      (Actor|DestroyActor))))

(fn ConstructionScript
  (|CallParentFunction))

(fn AddtoPlayerInventory
  (params (NewKey :type E_KeyTypes%20Enum :default "NewEnumerator3"))
  (return 0))

(fn GetPlayerInventory
  (return ""))