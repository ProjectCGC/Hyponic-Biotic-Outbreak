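; Health pickup token whose cross mesh spins and bobs, restoring the player's health when overlapped.
; A timeline drives the idle motion, resetting the cross to its cached transform each update before applying offsets.
; Player overlap stops the idle, calls EventHealthRestore on BP_Player and plays a Wwise sound guarded by DoOnce.
; A second timeline pulls the cross toward the player, and the actor destroys itself after a short delay.
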(event OnComponentBeginOverlap(Cross_Collision)
  (params (OverlappedComponent :type Primitive%20Component%20Object%20Reference) (OtherActor :type Actor%20Object%20Reference) (OtherComp :type Primitive%20Component%20Object%20Reference) (OtherBodyIndex :type Integer) (bFromSweep :type Boolean) (SweepResult :type Hit%20Result%20Structure%20%28by%20ref%29))
  ;[1 1 1] Token to Player Animation
  (if (== OtherActor (Game|Player|GetPlayerPawn 0))
    (Variables|Default|SetbAnimate false)
    (CallFunction|OnHealthRestore)
    (bind _move_to_player (Timeline|Token%20to%20Player%20Timeline Play)
      (:Update
        (bind _returnvalue (CallFunction|InterpolatetoPlayer _move_to_player))
        (Transformation|SetWorldLocation (Variables|Default|GetCross_Vertical) _returnvalue false false)
        (Utilities|FlowControl|Delay 1.0)
        (Actor|DestroyActor)))))

(event Custom|OnHealthRestore
  (bind _returnvalue (Game|Player|GetPlayerPawn 0))
  (bind _asbp_player (Utilities|Casting|CastToBP_Player _returnvalue))
  (Default|EventHealthRestore _asbp_player (Variables|Default|GetHealth%20Restore%20Delta))
  (Utilities|FlowControl|DoOnce false
    (:Completed
      ;[0 0 1] Audio
      (Default|PlayWwiseEvent (Variables|Default|GetAC_WwiseAudioComponent) (Variables|WwiseAudio|GetPlay_PLYR_HealthUp) _returnvalue))))

(event EventBeginPlay
  (bind _cross_vertical (Variables|Default|GetCross_Vertical))
  (bind _returnvalue (Transformation|GetRelativeTransform _cross_vertical))
  ;[1 1 1] Token Animations
  (CallFunction|SetOGVariables)
  (bind (_direction _rotating_progression _transform_progression) (Timeline|Timeline Play)
    (:Update
      (if (== (Variables|Default|GetbAnimate) true)
        (CallFunction|RestoreOGValues)
        (bind (_location _rotation _scale) (CallFunction|InterpolateTransform _rotating_progression _transform_progression))
        (Transformation|SetRelativeTransform (Variables|Default|GetCross_Vertical) (Math|Transform|MakeTransform (Math|Vector|Lerp(Vector) (.location _returnvalue) (+ (.location _returnvalue) _transform_progression) 1.0) _rotation _scale) false false)))))

(fn ConstructionScript)

(fn SetOGVariables
  (bind _cross_vertical (Variables|Default|GetCross_Vertical))
  (Variables|Default|SetCross%20OG%20Location (Transformation|GetWorldLocation _cross_vertical))
  (Variables|Default|SetCross%20OG%20Rotation (Transformation|GetWorldRotation _cross_vertical)))

(fn RestoreOGValues
  (bind _cross_vertical (Variables|Default|GetCross_Vertical))
  (Transformation|SetWorldLocation _cross_vertical (Variables|Default|GetCross%20OG%20Location) false false)
  (Transformation|SetWorldRotation _cross_vertical (Variables|Default|GetCross%20OG%20Rotation) false false))

(fn InterpolateTransform
  (params (Rotation%20In :type Float%20%28single-precision%29) (Location%20In :type Float%20%28double-precision%29))
  (bind _returnvalue (CallFunction|InterpolationRotation Rotation%20In))
  (bind _returnvalue_2 (CallFunction|InterpolateLocation Location%20In))
  (return _returnvalue_2 _returnvalue (Variables|/Script/Engine.SceneComponent|GetRelativeScale3D (Variables|Default|GetCross_Vertical))))

(fn InterpolationRotation
  (params (B_Yaw :type Float%20%28single-precision%29))
  (return (Math|Rotator|Lerp(Rotator) "0, 0, 0" (Math|Rotator|MakeRotator 0.0 0.0 B_Yaw) 1.0)))

(fn InterpolateLocation
  (params (A :type Float%20%28double-precision%29))
  (bind _cross_vertical (Variables|Default|GetCross_Vertical))
  (bind _returnvalue (Transformation|GetWorldLocation _cross_vertical))
  (return (Math|Vector|Lerp(Vector) "0, 0, 0" (Math|Vector|MakeVector (.x _returnvalue) (.y _returnvalue) (+ A (.z _returnvalue))) 1.0)))

(fn OnHungerReplenished)

(fn InterpolatetoPlayer
  (params (Alpha :type Float%20%28single-precision%29))
  (return (Math|Vector|Lerp(Vector) (Transformation|GetWorldLocation (Variables|Default|GetCross_Vertical)) (Transformation|GetActorLocation (Game|Player|GetPlayerPawn 0)) Alpha)))