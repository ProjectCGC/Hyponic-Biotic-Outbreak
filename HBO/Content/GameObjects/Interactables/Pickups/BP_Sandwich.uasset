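; BP_Sandwich is a sandwich pickup that animates its Sandwich component's height and spin; it contains no collection logic.
; BeginPlay caches the original transform and starts a Timeline with rotation and height tracks.
; Each update restores that transform, then sets yaw from the rotation track and offsets Z by the height track, so offsets never accumulate.
; The lerps use an alpha of 1, acting as direct sets, and every update calls Play again.
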(event EventBeginPlay
  (bind _sandwich (Variables|Default|GetSandwich))
  (bind _sandwich_2 (Variables|Default|GetSandwich))
  (bind _sandwich_3 (Variables|Default|GetSandwich))
  (bind _sandwich_4 (Variables|Default|GetSandwich))
  (bind _returnvalue (Transformation|GetWorldLocation _sandwich_4))
  (bind _returnvalue_2 (Transformation|GetWorldRotation _sandwich_3))
  (bind _output_get (Variables|Default|SetSandwich%20OG%20Location (Transformation|GetWorldLocation (Variables|Default|GetSandwich))))
  (bind _output_get_2 (Variables|Default|SetSandwich%20OG%20Rotation (Transformation|GetWorldRotation (Variables|Default|GetSandwich))))
  (Variables|Default|SetSandwich%20Z%20Rotation (.yaw _returnvalue_2))
  (Variables|Default|SetSandwich%20Y%20Rotation (.pitch _returnvalue_2))
  (Variables|Default|SetSandwich%20X%20Rotation (.roll _returnvalue_2))
  (bind (_direction _rotating_progression _transform_progression) (Timeline|Timeline Play)
    (:Update
      (Transformation|SetWorldLocation _sandwich_2 _output_get false false)
      (Transformation|SetWorldRotation _sandwich_2 _output_get_2 false false)
      (Transformation|SetWorldRotation (Variables|Default|GetSandwich) (Math|Rotator|Lerp(Rotator) (Transformation|GetWorldRotation (Variables|Default|GetSandwich)) (Math|Rotator|MakeRotator (Variables|Default|GetSandwich%20X%20Rotation) (Variables|Default|GetSandwich%20Y%20Rotation) _rotating_progression) 1.0) false false)
      (Transformation|SetWorldLocation _sandwich (Math|Vector|Lerp(Vector) (Transformation|GetWorldLocation _sandwich) (Math|Vector|MakeVector (.x _returnvalue) (.y _returnvalue) (+ _transform_progression (.z _returnvalue))) 1.0) false false)
      (Timeline|Timeline Play))))

(fn ConstructionScript)