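; Placeholder gun Blueprint handling hitscan shooting, timed reloads and aim-down-sights, with FMOD audio.
; Shoot checks reload, cooldown and ammo, line-traces from the camera with random bloom when not aiming, damages Enemy-tagged actors and spawns impact effects.
; It returns a result struct carrying reload requests and camera recoil to the caller.
; Timelines with ease-out smoothing animate the model's ADS movement and randomized recoil recovery.
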(event EventBeginPlay
  (bind _model (Variables|Default|GetModel))
  (bind _returnvalue (Transformation|GetRelativeTransform _model))
  (bind (_location _rotation) (Math|Transform|BreakTransform _returnvalue))
  ;[1 1 0.5] Initialize Original Pos and Rot
  (Variables|Properties|SetOriginalLocation _location)
  (Variables|Properties|SetOriginalRotation _rotation)
  ;[1 1 0.5] Prepare Timelines
  (Components|Timeline|SetPlayRate (Variables|Default|GetADSTimeline) (/ 1.0 (Variables|ADS|GetADSTime)))
  (Components|Timeline|SetPlayRate (Variables|Default|GetRecoilTimeline) (/ 1.0 (Variables|Recoil|GetRecoveryTime))))

(event EventReload
  (bind _debugmessages (Variables|Properties|GetDebugMessages))
  ;[1 1 0.5] Reload Sequence
  (if (not (Variables|State|GetReloading))
    (Utilities|FlowControl|Sequence
      (:then_0
        (CallFunction|ADS false) ; Exit ADS BEFORE setting reload
        (Variables|State|SetReloading true))
      (:then_1
        (Utilities|Time|SetTimerbyFunctionName 0 "FinishReload" (Variables|Properties|GetReloadTime)))
      (:then_2
        ;;[0 0 1] Play Reload Sound
        (if (Variables|Properties|GetDebugPlaySounds)
          (Default|PlayFMODEvent (Variables|Default|GetAC_FMODAudioComponent) (Variables|Audio|GetReloadAudioEvent))))
      (:then_3
        (Development|PrintString "Start Reload" _debugmessages _debugmessages) ; Replace with UI Events
      ))))

(event EventADS
  (params (Aiming :type Boolean))
  (bind _ac_fmodaudiocomponent (Variables|Default|GetAC_FMODAudioComponent))
  (if (not (Variables|State|GetReloading)) ; Ignore ADS events while reloading
    (bind _output_get (Variables|State|SetAiming Aiming))
    (Utilities|FlowControl|Sequence
      (:then_0
        ;[1 1 0.5] ADS Animation
        (Variables|ADS|SetAimingChangePosition (.Location (Math|Transform|BreakTransform (Transformation|GetRelativeTransform (Variables|Default|GetModel))))) ; Set where the ADS animation stops
        (bind _adsanimpercentage (Timeline|ADSTimeline PlayFromStart)
          (:Update
            (bind _output_get_2 (Variables|State|SetTargetLocation (Math|Vector|Lerp(Vector) (Variables|ADS|GetAimingChangePosition) (select (Variables|State|GetAiming) (Variables|ADS|GetADSPos) (Variables|Properties|GetOriginalLocation)) (Utilities|MPercenttoSmoothedPercent _adsanimpercentage))))
            (Transformation|SetRelativeLocation (Variables|Default|GetModel) _output_get_2 false false))))
      (:then_1
        ;[0 0 1] Play ADS Sounds
        (if (Variables|Properties|GetDebugPlaySounds)
          (if _output_get
            (Default|PlayFMODEvent _ac_fmodaudiocomponent (Variables|Audio|GetADSStartAudioEvent))
            (else
              (Default|PlayFMODEvent _ac_fmodaudiocomponent (Variables|Audio|GetADSEndAudioEvent)))))))))

(fn ConstructionScript)

(fn ShootFunc
  (params (Player :type Actor%20Object%20Reference) (Camera :type Scene%20Component%20Object%20Reference))
  (bind (_startpoint _endpoint) (|GetCastPoints Camera))
  (bind _s_shootresult (|EmptyResult))
  (bind (_positionrecoil _rotationrecoil) (Utilities|MGetGunRecoil))
  (bind _debugmessages (Variables|Properties|GetDebugMessages))
  ;[1 1 0.5] Conditions to Shoot: Not reloading, >0 Ammo, Not on Shoot Cooldown
  (if (Variables|State|GetReloading)
    (return _s_shootresult)
    (elif (Variables|State|GetShootCooldown)
      (return _s_shootresult)
      (elif (> (Variables|State|GetAmmo) 0)
        (bind (_outhit _returnvalue) (Collision|LineTraceByChannel _startpoint (+ _endpoint (|GetBloomComponent Camera)) "TraceTypeQuery1" false (Utilities|Array|MakeArray Player) "ForDuration" true "(R=1.000000,G=0.000000,B=0.000000,A=1.000000)" "(R=0.000000,G=1.000000,B=0.000000,A=1.000000)" 2.0))
        (Utilities|FlowControl|Sequence
          (:then_0
            ;[1 1 0.5] Administer Damage
            (if _returnvalue ; If something was hit
              (if (Actor|ActorHasTag (.HitActor (Collision|BreakHitResult _outhit)) "Enemy")
                (Game|Damage|ApplyDamage (.HitActor (Collision|BreakHitResult _outhit)) (Variables|Properties|GetDamage) 0 0) ; This needs to be implemented in the Enemy blueprint to function, as it calls an event for the enemy.
              )))
          (:then_1
            ;[1 1 0.5] Decrement Ammo
            (bind _result (Math|Integer|DecrementInt (Variables|State|GetAmmo))
              (:%20%20
                (bind _output_get (Variables|State|SetAmmo _result))
                (Development|PrintString (Utilities|String|Append "Ammo: " (Utilities|String|ToString(Integer) _output_get)) _debugmessages _debugmessages "(R=0.000000,G=0.660000,B=1.000000,A=1.000000)" 1.0))))
          (:then_2
            ;[1 1 0.5] Set Cooldown
            (Utilities|Time|SetTimerbyFunctionName 0 "ReleaseCooldown" (/ (Math|Conversions|ToFloat(Integer) (Variables|Properties|GetFirerate)) 6e+01)))
          (:then_3
            ;[0 0 1] Play Gunshot Sound
            (if (Variables|Properties|GetDebugPlaySounds)
              (Default|PlayFMODEvent (Variables|Default|GetAC_FMODAudioComponent) (Variables|Audio|GetGunshotAudioEvent))))
          (:then_4
            ;[1 1 0.5] Activate Particles
            (Niagara|ResetSystem (Variables|Default|GetMuzzleFlash))
            (if (Actor|ActorHasTag (.HitActor (Collision|BreakHitResult _outhit)) "Enemy")
              (LocalVariables|SetParticleToSpawn "/Game/Effects/FXS_BulletImpactFlesh.FXS_BulletImpactFlesh")
              (else
                (LocalVariables|SetParticleToSpawn "/Game/Effects/FXS_BulletImpactConcrete.FXS_BulletImpactConcrete")))
            (Niagara|SpawnSystematLocation (LocalVariables|GetParticleToSpawn) (.Location (Collision|BreakHitResult _outhit)) (Math|Rotator|MakeRotfromX (.Normal (Collision|BreakHitResult _outhit)))))
          (:then_5
            ;[1 1 0.5] Set Recoil
            (Variables|State|SetLastRecoilOffset _positionrecoil)
            (Variables|State|SetLastRecoilRotation _rotationrecoil)
            (Components|Timeline|PlayfromStart (Variables|Default|GetRecoilTimeline)))
          (:then_6
            ;[1 1 0.5] Return Shoot Result
            (return (Utilities|Struct|MakeS_ShootResult false (Variables|State|GetAiming) (Utilities|MGetCameraRecoil)))))
        (else
          (return (|ReloadResult)))))))

(fn FinishReload
  (bind _debugmessages (Variables|Properties|GetDebugMessages))
  (bind _output_get (Variables|State|SetAmmo (Variables|Properties|GetClipSize)))
  (Variables|State|SetReloading false)
  (Development|PrintString (Utilities|String|Append "Reloaded, Ammo: " (Utilities|String|ToString(Integer) _output_get)) _debugmessages _debugmessages))

(fn ReleaseCooldown
  (Variables|State|SetShootCooldown false))

(fn Shoot
  (params (Player :type Actor%20Object%20Reference) (Camera :type Scene%20Component%20Object%20Reference))
  (bind _shootresult (CallFunction|ShootFunc Player Camera))
  (return _shootresult))