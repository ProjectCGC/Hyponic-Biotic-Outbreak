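; BP_Door is a sliding door barrier that toggles open and closed when it receives an InteractComplete pulse from its associated BP_Button.
; A Finished flag blocks retriggering while the DoorAnim timeline lerps the actor from its current transform toward an offset set by DoorSettings.
; A macro builds the slide direction from local forward, right and up axes, and IsClosed, flipped on completion, picks the sign.
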(event EventInteractComplete
  (params (Interactee :type Actor%20Object%20Reference%20%28by%20ref%29) (PlayerInventory :type F%20Player%20Inventory%20Structure%20%28by%20ref%29))
  (bind _returnvalue (Transformation|GetActorTransform))
  (bind (_doorsettings _doorsettings_slidedirection_z _doorsettings_slidedirection_y _doorsettings_slidedirection_x) (Variables|Default|GetDoorSettings))
  ;[0.18 0.3 0.3] Barrier Object Received Pulse From Associated BP_Button
  (if (Variables|Default|GetFinished)
    (Variables|Default|SetFinished false)
    ;;[0.07158 0.2812 0.256] Door Motion
    (bind _slidingdoor (Timeline|DoorAnim PlayFromStart)
      (:Update
        (Transformation|SetActorTransform (Math|Transform|Lerp(Transform) (Transformation|GetActorTransform) (Math|Transform|MakeTransform (+ (* (Math|Float|SelectFloat (.slidedistance _doorsettings) (* -1.0 (.slidedistance _doorsettings)) (Variables|Default|GetIsClosed)) (Utilities|MLocalVectfromBool _doorsettings_slidedirection_x _doorsettings_slidedirection_y _doorsettings_slidedirection_z)) (.location _returnvalue)) (.rotation _returnvalue) (.scale _returnvalue)) _slidingdoor)))
      (:Finished
        (Variables|Default|SetFinished true)
        (Variables|Default|SetIsClosed (not (Variables|Default|GetIsClosed)))))))

(fn ConstructionScript)