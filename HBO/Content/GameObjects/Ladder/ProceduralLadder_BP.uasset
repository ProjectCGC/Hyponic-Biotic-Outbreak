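; ProceduralLadder_BP is a procedural ladder actor that builds itself to a configurable height in the Construction Script.
; It scales the two side poles to LadderHeight, then loops AddBarsAndScrews, placing rungs at LadderGap spacing until the height is reached.
; Rungs and optional screw pairs, added every ScrewInterval rungs, are instances on separate instanced mesh components.
; The Event Graph holds no gameplay logic.
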(event EventBeginPlay)

(event Collision|EventActorBeginOverlap
  (params (OtherActor :type Actor%20Object%20Reference)))

(event EventTick
  (params (DeltaSeconds :type Float%20%28single-precision%29)))

(fn ConstructionScript
  (Transformation|SetRelativeScale3D (Variables|Default|GetLeftLadderPole) (Math|Vector|MakeVector 0.1 0.1 (Variables|Default|GetLadder%20Height)))
  (while (< (Variables|Default|GetCompareHeight) (* (Variables|Default|GetLadder%20Height) 1e+02))
    (Utilities|AddBarsandScrews)))