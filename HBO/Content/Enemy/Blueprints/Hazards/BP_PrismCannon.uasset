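; BP_PrismCannon is an enemy hazard cannon that automatically fires projectiles at a fixed interval for as long as it is in play.
; BeginPlay starts an endless Delay loop that waits FireRate seconds before each shot.
; Each shot passes through SpawnProjectiles to ShootTestProjectiles, which spawns a BP_TestProjectile at the Arrow component's location and rotation, scaled uniformly by ProjectileSize.
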(event EventBeginPlay
  ;[1 0.2174 0.3473] Projectile Loop
  (Utilities|FlowControl|Delay (Variables|Default|GetFire%20Rate) :!label _label)
  (CallFunction|SpawnProjectiles (Variables|Default|GetProjectile%20Size))
  (goto _label))

(event Collision|EventActorBeginOverlap
  (params (OtherActor :type Actor%20Object%20Reference)))

(event EventTick
  (params (DeltaSeconds :type Float%20%28single-precision%29)))

(fn ConstructionScript)

(fn SpawnProjectiles
  (params (Projectile%20Size :type Float%20%28double-precision%29))
  (CallFunction|ShootTestProjectiles Projectile%20Size))

(fn ShootTestProjectiles
  (params (Projectile%20Size :type Float%20%28double-precision%29))
  (Game|SpawnActorfromClass "/Game/Enemy/Blueprints/Hazards/Projectiles/BP_TestProjectile.BP_TestProjectile_C" (Math|Transform|MakeTransform (Transformation|GetWorldLocation (Variables|Default|GetArrow)) (Transformation|GetWorldRotation (Variables|Default|GetArrow)) (Math|Conversions|ToVector(Float) Projectile%20Size)) "Undefined" "MultiplyWithRoot" 0 0))