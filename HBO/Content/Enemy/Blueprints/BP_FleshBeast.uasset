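; FleshBeast enemy Blueprint that serves its AI controller and behavior tree with attacks, movement speeds, patrol points and wander data.
; Attack requests damage player pawn 0 without a range check, then report success after a delay.
; State updates set walk speed from MoveData and reply whether it changed, though getter and setter disagree on Investigating speed.
; GetEnemyState always returns Idle.
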(event EventUpdatebyState
  (params (EnemyState :type E_EnemyState%20Enum%20%28by%20ref%29 :default "NewEnumerator0"))
  (bind _returnvalue (Pawn|GetController))
  ;[0.18 0.3 0.3] Communication with AI Controller
  ;;[0.1 0.2 0.2] Update Move Speed by State
  (bind _speed (CallFunction|GetSpeedbyState EnemyState))
  (if (Math|Float|NearlyEqual(Float) _speed (Class|MovementComponent|GetMaxSpeed (Variables|Character|GetCharacterMovement)) 0.001)
    (Class|BPIAI|Succeeded(Message) _returnvalue false)
    (else
      (CallFunction|SetSpeedbyState EnemyState)
      (Class|BPIAI|Succeeded(Message) _returnvalue true))))

(event EventInitiateAttack
  (params (RequestedBy :type Object%20Object%20Reference%20%28by%20ref%29))
  ;[0.18 0.3 0.3] Direct Communication with Behavior Tree
  ;;[0.1 0.2 0.2] Initiate Attack from BT
  (Game|Damage|ApplyDamage (Game|Player|GetPlayerPawn 0) (Variables|AI|GetBasicAttackDmg) 0 0)
  (Utilities|FlowControl|Delay (Variables|AI|GetBasicAttackDelay))
  (Class|BPIAI|Succeeded(Message) RequestedBy true))

(fn ConstructionScript)

(fn SetSpeedbyState
  (params (State :type E_EnemyState%20Enum :default "NewEnumerator0"))
  (bind _movedata (Variables|AI|GetMoveData))
  (Variables|/Script/Engine.CharacterMovementComponent|SetMaxWalkSpeed (Variables|Character|GetCharacterMovement) (Utilities|Select :Index State :NewEnumerator0 (.idlespeed _movedata) :NewEnumerator1 (.wanderspeed _movedata) :NewEnumerator2 (.patrolspeed _movedata) :NewEnumerator3 (.idlespeed _movedata) :NewEnumerator4 (.patrolspeed _movedata) :NewEnumerator5 (.combatspeed _movedata))))

(fn GetSpeedbyState
  (params (State :type E_EnemyState%20Enum :default "NewEnumerator0"))
  (bind _movedata (Variables|AI|GetMoveData))
  (return (Utilities|Select :Index State :NewEnumerator0 (.idlespeed _movedata) :NewEnumerator1 (.wanderspeed _movedata) :NewEnumerator2 (.patrolspeed _movedata) :NewEnumerator3 (.idlespeed _movedata) :NewEnumerator4 (.wanderspeed _movedata) :NewEnumerator5 (.combatspeed _movedata))))

(fn GetEnemyState
  (return "NewEnumerator0"))

(fn RequestPatrolPoints
  (bind _patrolroute (Variables|AI|GetPatrolRoute))
  (Utilities|IsValid _patrolroute
    (:Is%20Valid
      (bind _patrolpoints (Default|GetPatrolPoints _patrolroute))
      (return _patrolpoints))
    (:Is%20Not%20Valid
      (return 0))))

(fn RequestWanderData
  (return (Variables|AI|GetWanderData)))