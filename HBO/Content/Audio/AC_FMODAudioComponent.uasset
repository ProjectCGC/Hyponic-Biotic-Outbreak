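; Audio component that wraps FMOD Studio calls for game audio, exposing typed events for setting music and sound parameters and a helper for playing events.
; Area, zone, menu and combat state and intensity are written as global FMOD parameters.
; Ground material and clamped 0–1 movement speed are set on a given event instance.
; PlayFMODEvent attaches an event to a valid target actor's root component and returns it.
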(event Custom|Set%20FMOD%20Parameter%20-%20Zone%20State
  (params (Zone%20State :type E_ZoneState%20Enum :default "NewEnumerator0"))
  ;[0 0 1] Set FMOD Parameter
  (Class|FMODBlueprintStatics|SetGlobalParameterbyName "ZoneState" (Math|Conversions|ToFloat(Byte) Zone%20State)))

(event Custom|Set%20FMOD%20Parameter%20-%20Ground%20Material
  (params (FMOD%20Event :type FMOD%20Audio%20Component%20Object%20Reference) (GroundMaterial :type E_CombatState%20Enum :default "NewEnumerator0"))
  ;[0 0 1] Set FMOD Parameter
  (Class|FMODAudioComponent|SetParameter FMOD%20Event "GroundMaterial" (Math|Conversions|ToFloat(Byte) GroundMaterial)))

(event Custom|Set%20FMOD%20Parameter%20-%20MovementSpeed
  (params (EventInstance :type FMOD%20Audio%20Component%20Object%20Reference) (MovementSpeed :type Float%20%28double-precision%29))
  ;[0 0 1] Set FMOD Parameter
  (Class|FMODAudioComponent|SetParameter EventInstance "MovementSpeed" (Math|Float|Clamp(Float) MovementSpeed)))

(event Custom|Set%20FMOD%20Parameter%20-%20Combat%20State
  (params (CombatState :type E_CombatState%20Enum :default "NewEnumerator0"))
  ;[0 0 1] Set FMOD Parameter
  (Class|FMODBlueprintStatics|SetGlobalParameterbyName "CombatState" (Math|Conversions|ToFloat(Byte) CombatState)))

(event Custom|Set%20FMOD%20Parameter%20-%20Menu%20State
  (params (Menu%20State :type E_MenuState%20Enum :default "NewEnumerator0"))
  ;[0 0 1] Set FMOD Parameter
  (Class|FMODBlueprintStatics|SetGlobalParameterbyName "MenuState" (Math|Conversions|ToFloat(Byte) Menu%20State)))

(event Custom|Set%20FMOD%20Parameter%20-%20Area%20State
  (params (AreaState :type E_AreaState%20Enum :default "NewEnumerator0"))
  ;[0 0 1] Set FMOD Parameter
  (Class|FMODBlueprintStatics|SetGlobalParameterbyName "AreaState" (Math|Conversions|ToFloat(Byte) AreaState)))

(event Custom|Set%20FMOD%20Parameter%20-%20Combat%20Intensity
  (params (CombatIntensity :type E_CombatIntensity%20Enum :default "NewEnumerator0"))
  ;[0 0 1] Set FMOD Parameter
  (Class|FMODBlueprintStatics|SetGlobalParameterbyName "CombatIntensity" (Math|Conversions|ToFloat(Byte) CombatIntensity)))

(fn PlayFMODEvent
  (params (Event :type FMOD%20Event%20Object%20Reference) (Target%20Actor :type Actor%20Object%20Reference))
  ;[0 0 1] Play FMOD Event
  (Utilities|IsValid Target%20Actor
    (:Is%20Valid
      (bind _returnvalue (Class|FMODBlueprintStatics|PlayEventAttached Event (Variables|/Script/Engine.Actor|GetRootComponent Target%20Actor) "None" "0, 0, 0" "KeepRelativeOffset"))
      (return _returnvalue))))